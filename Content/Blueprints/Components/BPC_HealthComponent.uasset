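; Health component that stores current and max health for its owning actor.
; InitHealth fills health to the given max, with getters exposing both values.
; Decrease and increase functions clamp health between zero and max and broadcast OnUpdateHealth, though increases pass 0 instead of the new value.
; Reaching zero fires OnDie and blocks further damage; death and every increase print debug text with the owner's name.
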(event EventBeginPlay)

(event EventTick
  (params (DeltaSeconds :type Float%20%28single-precision%29)))

(fn InitHealth
  (params (MaxHealth :type Float%20%28double-precision%29))
  (bind _output_get (Variables|Default|SetMaxHealth MaxHealth))
  (Variables|Default|SetHealth _output_get))

(fn DecreaseHealth
  (params (Value :type Float%20%28double-precision%29))
  (if (> (Variables|Default|GetHealth) 0.0)
    (bind _output_get (Variables|Default|SetHealth (Math|Float|Max(Float) (- (Variables|Default|GetHealth) Value) 0.0)))
    (Default|CallOnUpdateHealth _output_get)
    (if (<= (Variables|Default|GetHealth) 0.0)
      (Default|CallOnDie 0.0)
      (Development|PrintText (Utilities|Text|FormatText "{Owner} Decrae Health : {Value}" (Utilities|GetObjectName (Components|GetOwner)) (Variables|Default|GetHealth))))))

(fn IncreaseHealth
  (params (Value :type Float%20%28double-precision%29))
  (Variables|Default|SetHealth (Math|Float|Min(Float) (+ (Variables|Default|GetHealth) Value) (Variables|Default|GetMaxHealth)))
  (Default|CallOnUpdateHealth 0.0)
  (Development|PrintText (Utilities|Text|FormatText "{Owner} Increase Health : {Value}" (Utilities|GetObjectName (Components|GetOwner)) (Variables|Default|GetHealth))))

(fn GetHealth
  (return (Variables|Default|GetHealth)))

(fn GetMaxHealth
  (return (Variables|Default|GetMaxHealth)))