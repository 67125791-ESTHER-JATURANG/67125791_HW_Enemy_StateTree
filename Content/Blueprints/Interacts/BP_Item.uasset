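; BP_Item is an interactable item actor that shows a "Collect Item" prompt.
; On interact, it runs the parent logic, then plays the reach-lever montage on the interactor's mesh.
; IsInteract is cleared when the montage completes or is interrupted.
; The graph itself has no pickup, inventory or destroy logic.
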(event EventBeginPlay
  (|CallParentFunction) ; This node is disabled and will not be called.\nDrag off pins to build functionality.
)

(event Collision|EventActorBeginOverlap
  (params (OtherActor :type Actor%20Object%20Reference))
  (|CallParentFunction OtherActor) ; This node is disabled and will not be called.\nDrag off pins to build functionality.
)

(event EventTick
  (params (DeltaSeconds :type Float%20%28single-precision%29))
  (|CallParentFunction DeltaSeconds) ; This node is disabled and will not be called.\nDrag off pins to build functionality.
)

(event EventOnInteract
  (params (Interactor :type BP%20Player%20Character%20Object%20Reference))
  (|CallParentFunction Interactor)
  (Animation|Montage|PlayMontage (Variables|/Script/Engine.Character|GetMesh Interactor) "/Game/Assets/Animations/AM_ReachLever_Montage.AM_ReachLever_Montage"
    (:OnCompleted
      _)
    (:OnInterrupted
      _))
  (Variables|Default|SetIsInteract false))

(fn ConstructionScript
  (|CallParentFunction))

(fn GetInteractText
  (return "Collect Item"))