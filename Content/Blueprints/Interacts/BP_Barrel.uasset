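; BP_Barrel is a barrel actor that damages itself when the third-person character enters its sphere trigger.
; A health component is initialized on BeginPlay, and the AnyDamage event passes incoming damage to it.
; The overlap damage equals the starting health, so one touch is enough to deplete it.
; The branch after the health read leads to no action, so this graph implements no destruction or explosion.
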(event OnComponentBeginOverlap(Sphere1)
  (params (OverlappedComponent :type Primitive%20Component%20Object%20Reference) (OtherActor :type Actor%20Object%20Reference) (OtherComp :type Primitive%20Component%20Object%20Reference) (OtherBodyIndex :type Integer) (bFromSweep :type Boolean) (SweepResult :type Hit%20Result%20Structure%20%28by%20ref%29))
  (Utilities|Casting|CastToBP_ThirdPersonCharacter OtherActor)
  (Game|Damage|ApplyDamage self 1e+02 0 0))

(event EventBeginPlay
  (|CallParentFunction)
  (Default|InitHealth (Variables|Default|GetBPC_HealthComponent) 1e+02))

(event Game|Damage|EventAnyDamage
  (params (Damage :type Float%20%28single-precision%29) (DamageType :type Damage%20Type%20Object%20Reference) (InstigatedBy :type Controller%20Object%20Reference) (DamageCauser :type Actor%20Object%20Reference))
  (Default|DecreaseHealth (Variables|Default|GetBPC_HealthComponent) Damage)
  (Default|GetHealth (Variables|Default|GetBPC_HealthComponent))
  (if true
    _))

(event EventTick
  (params (DeltaSeconds :type Float%20%28single-precision%29)))

(event Collision|EventActorBeginOverlap
  (params (OtherActor :type Actor%20Object%20Reference)))

(fn ConstructionScript)