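; Health component that tracks an owning actor's current health and death state.
; On BeginPlay it fills health to the maximum, broadcasts the change and binds to the owner's OnTakeAnyDamage event.
; Damage passes to ApplyDamageAmount, which ignores dead owners, clamps health, broadcasts and prints the new value.
; When health reaches zero, it sets IsDead and fires the OnDeath dispatcher once.
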(event Custom|HandleAnyDamage
  (params (DamagedActor :type Actor%20Object%20Reference) (Damage :type Float%20%28single-precision%29) (DamageType :type Damage%20Type%20Object%20Reference) (InstigatedBy :type Controller%20Object%20Reference) (DamageCauser :type Actor%20Object%20Reference))
  (CallFunction|ApplyDamageAmount Damage))

(event EventBeginPlay
  (Variables|Default|SetCurrentHealth (Variables|Default|GetMaxHealth))
  (Default|CallOnHealthChanged (Variables|Default|GetCurrentHealth) (Variables|Default|GetMaxHealth))
  (EventDispatchers|AssignOnTakeAnyDamage (Components|GetOwner) (delegate Custom|HandleAnyDamage)))

(event EventTick
  (params (DeltaSeconds :type Float%20%28single-precision%29)))

(fn ApplyDamageAmount
  (params (Amount :type Float%20%28double-precision%29))
  (if (not (Variables|Default|GetIsDead))
    (Variables|Default|SetCurrentHealth (Math|Float|Clamp(Float) (- (Variables|Default|GetCurrentHealth) Amount) 0.0 (Variables|Default|GetMaxHealth)))
    (Default|CallOnHealthChanged (Variables|Default|GetCurrentHealth) (Variables|Default|GetMaxHealth))
    (Development|PrintString (Utilities|String|ToString(Float) (Variables|Default|GetCurrentHealth)))
    (if (<= (Variables|Default|GetCurrentHealth) 0.0)
      (Variables|Default|SetIsDead true)
      (Default|CallOnDeath))))