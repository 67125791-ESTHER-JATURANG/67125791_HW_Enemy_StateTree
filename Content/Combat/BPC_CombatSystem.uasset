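; Combat component for a Character owner that runs montage-based melee attacks and applies hit damage.
; BeginAttackEvent plays the attack montage if not already attacking, reports completion or interruption via CallOnAttackFinish, then EndAttackEvent clears the flag and stops the montage.
; TraceHit sphere-overlaps pawns, ignoring the owner, and damages each only once, tracked in HitActors until ResetHitActors clears it.
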(event Custom|BeginAttackEvent
  (if (not (Variables|Default|GetIsAttacking))
    (Animation|Montage|PlayMontage (Variables|/Script/Engine.Character|GetMesh (Variables|Default|GetOwnerCharacter%20)) (Variables|Default|GetAttackMontage)
      (:then
        (Variables|Default|SetIsAttacking true)
        (Variables|Default|SetLastAttackMontage (Variables|Default|GetAttackMontage)))
      (:OnCompleted
        (Default|CallOnAttackFinish true)
        (CallFunction|EndAttackEvent))
      (:OnInterrupted
        (Default|CallOnAttackFinish false)
        (CallFunction|EndAttackEvent)))))

(event Custom|EndAttackEvent
  (Utilities|FlowControl|Sequence
    (:then_0
      (if (Variables|Default|GetIsAttacking)
        (Variables|Default|SetIsAttacking false)))
    (:then_1
      (Utilities|IsValid (Variables|Default|GetLastAttackMontage)
        (:Is%20Valid
          (Animation|Montage|MontageStop (Components|SkeletalMesh|GetAnimInstance (Variables|/Script/Engine.Character|GetMesh (Variables|Default|GetOwnerCharacter%20))) 0.0 (Variables|Default|GetLastAttackMontage)))))))

(event EventBeginPlay
  (bind _ascharacter (Utilities|Casting|CastToCharacter (Components|GetOwner)))
  (CallFunction|SetOwnerCharacter _ascharacter))

(event EventTick
  (params (DeltaSeconds :type Float%20%28single-precision%29)))

(fn SetOwnerCharacter
  (params (NewOwner :type Character%20Object%20Reference))
  (Variables|Default|SetOwnerCharacter%20 NewOwner))

(fn GetOwnerCharacter)

(fn ResetHitActors
  (Utilities|Array|Clear (Variables|Default|GetHitActors)))

(fn TraceHit
  (params (Location :type Vector) (Radius :type Float%20%28double-precision%29) (Damage :type Float%20%28double-precision%29))
  (bind _outactors (Collision|SphereOverlapActors Location Radius (Utilities|Array|MakeArray "ObjectTypeQuery3") 0 (Utilities|Array|MakeArray (Variables|Default|GetOwnerCharacter%20))))
  (for _array_element _outactors
    (if (not (Utilities|Array|ContainsItem (Variables|Default|GetHitActors) _array_element))
      (Utilities|Array|AddUnique (Variables|Default|GetHitActors) _array_element)
      (Game|Damage|ApplyDamage _array_element Damage (Pawn|GetController (Variables|Default|GetOwnerCharacter%20)) (Variables|Default|GetOwnerCharacter%20)))))